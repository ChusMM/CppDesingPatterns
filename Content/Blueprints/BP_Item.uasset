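; BP_Item is a spinning pickup that destroys itself and plays an eating sound when any actor overlaps it.
; On BeginPlay it constructs its own Subject and registers the custom GameState's AchievementManager on it, following the Observer pattern.
; Tick rotates the skeletal mesh by RotationSpeed per frame, and the overlap handler sends no notification to the Subject.
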(event `self.ReceiveBeginPlay`
  ;[1 1 1] Makes the AchievementManager to observe this item
  (bind _returnvalue (`|GenericCreateObject` "/Script/CppDesignPatterns.Subject" self))
  (set `self.ItemSubject` _returnvalue)
  (bind _ascustom_game_state_base (cast `CustomGameStateBase` (`GameplayStatics.GetGameState`)))
  (bind _returnvalue_2 (`CustomGameStateBase.GetAchievementManager` _ascustom_game_state_base))
  (`Subject.AddObserver` (`self.ItemSubject`) _returnvalue_2))

(event `self.ReceiveTick`
  (params (DeltaSeconds :type "Float (single-precision)"))
  (`SceneComponent.K2_AddLocalRotation` (`self.SkeletalMesh`) (`self.RotationSpeed`) false true))

(event `self.ReceiveActorBeginOverlap`
  (params (OtherActor :type "Actor Object Reference"))
  (`self.K2_DestroyActor`)
  (`GameplayStatics.PlaySound2D` "/Game/Audio/eating.Eating"))

(fn `UserConstructionScript`)